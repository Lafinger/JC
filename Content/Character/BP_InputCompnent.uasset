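; Input component that handles mouse look and movement for its owning pawn using Enhanced Input.
; On BeginPlay it caches the owner as a Pawn and adds the default mapping context to player 0's local input subsystem.
; The look action feeds controller yaw and pitch, while the move action adds movement input along the actor's right and forward vectors.
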(event Input|EnhancedActionEvents|EnhancedInputActionIA_Look_Mouse
  (params (ActionValue :type Vector%202D%20Structure) (ElapsedSeconds :type Float%20%28double-precision%29) (TriggeredSeconds :type Float%20%28double-precision%29) (InputAction :type Input%20Action%20Object%20Reference :default "/Game/Input/Actions/IA_Look_Mouse.IA_Look_Mouse"))
  (:Triggered
    (bind _playerpawn (Variables|Default|GetPlayerPawn)
      (:then
        (Pawn|Input|AddControllerYawInput _playerpawn (.x ActionValue))
        (Pawn|Input|AddControllerPitchInput _playerpawn (.y ActionValue)))
      (:else))))

(event Input|EnhancedActionEvents|EnhancedInputActionIA_Move
  (params (ActionValue :type Vector%202D%20Structure) (ElapsedSeconds :type Float%20%28double-precision%29) (TriggeredSeconds :type Float%20%28double-precision%29) (InputAction :type Input%20Action%20Object%20Reference :default "/Game/Input/Actions/IA_Move.IA_Move"))
  (:Triggered
    (bind _playerpawn (Variables|Default|GetPlayerPawn)
      (:then
        (Pawn|Input|AddMovementInput _playerpawn (Transformation|GetActorRightVector _playerpawn) (.x ActionValue) false)
        (Pawn|Input|AddMovementInput _playerpawn (Transformation|GetActorForwardVector _playerpawn) (.y ActionValue) false))
      (:else))))

(event EventBeginPlay
  (bind _aspawn (Utilities|Casting|CastToPawn (Components|GetOwner)))
  (Variables|Default|SetPlayerPawn _aspawn)
  (Input|AddMappingContext (PlayerController|LocalPlayerSubsystems|GetEnhancedInputLocalPlayerSubsystem (Game|GetPlayerController 0)) "/Game/Input/IMC_Default.IMC_Default" 0 "(bIgnoreAllPressedKeysUntilRelease=True,bForceImmediately=False)"))

(event EventTick
  (params (DeltaSeconds :type Float%20%28single-precision%29)))